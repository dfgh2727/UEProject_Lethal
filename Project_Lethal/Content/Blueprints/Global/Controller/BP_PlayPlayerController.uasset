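; BP_PlayPlayerController is a player controller that applies input and camera setup for play, with its steps commented as temporary.
; On BeginPlay it switches to game-only input, hides the mouse cursor and clamps the camera manager's view pitch range.
; Its SetupInputComponentEvent registers the IC_CharacterInput mapping context through an AddMappingContext call, leaving a direct Enhanced Input subsystem call unconnected.
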(event `self.ReceiveBeginPlay`
  (bind _returnvalue (`GameplayStatics.GetPlayerCameraManager` 0))
  (`|ExecutionSequence`
    (:`then_0`
      ; SetInputMode(임시)
      (`WidgetBlueprintLibrary.SetInputMode_GameOnly` self)
      (set `self.bShowMouseCursor` false))
    (:`then_1`
      ; SetPlayerCameraPitch(임시)
      (set `PlayerCameraManager.ViewPitchMin` -30.0 _returnvalue))
    (:`then_2`
      (set `PlayerCameraManager.ViewPitchMax` 20.0 _returnvalue))))

(event `self.SetupInputComponentEvent`
  ; MappingContexts(임시)
  (`self.AddMappingContext` "/Game/Blueprints/Character/Input/IC_CharacterInput.IC_CharacterInput"))

(fn `UserConstructionScript`)